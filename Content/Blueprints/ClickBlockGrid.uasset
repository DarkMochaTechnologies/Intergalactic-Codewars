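; ClickBlockGrid is a grid actor that spawns a square field of ClickBlock actors and keeps the score.
; Tick waits for a valid MainSpaceship, then DoOnce lays out Size×Size blocks from the actor's location using index division and modulo.
; Each block receives the grid, spaceship, its number and transform.
; AddScore increments Score and updates ScoreText, while GetGridBlock is an empty stub.
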(event `self.ReceiveTick`
  (params (DeltaSeconds :type "Float (single-precision)"))
  (bind _size (`self.Size`))
  (bind _blockspacing (`self.BlockSpacing`))
  ;[1 1 1] Spawn blocks
  (`/Engine/EditorBlueprintResources/StandardMacros.IsValid` (`self.Main Spaceship`)
    (:`Is Valid`
      (`/Engine/EditorBlueprintResources/StandardMacros.DoOnce` false
        (:`Completed`
          (bind _output_get (set `self.TotalSize` (- (* (`self.Size`) (`self.Size`)) 1)))
          (for _index (range (+ _output_get 1))
            (set `self.SetBlockNumber` _index)
            (bind _returnvalue (`KismetMathLibrary.Conv_VectorToTransform` (+ (`KismetMathLibrary.MakeVector` (* (/ _index _size) _blockspacing) (* (mod _index _size) _blockspacing)) (`self.K2_GetActorLocation`))))
            (bind _returnvalue_2 (`|SpawnActorFromClass` "/Game/Blueprints/ClickBlock.ClickBlock_C" _returnvalue false self)) ; Spawn a  block
            (bind _asclick_block (cast `/Game/Blueprints/ClickBlock` _returnvalue_2))
            (set `/Game/Blueprints/ClickBlock.Location` _returnvalue _asclick_block)
            (set `/Game/Blueprints/ClickBlock.MainSpaceship` (`self.Main Spaceship`) _asclick_block)
            (set `/Game/Blueprints/ClickBlock.ClickBlockNumber` (`self.SetBlockNumber`) _asclick_block)))))))

(event `AddScore`
  ;[1 1 1] Handle scoring when block is clicked
  (set `self.Score` (+ (`self.Score`) 1)) ; Increment score
  (`TextRenderComponent.SetText` (`self.ScoreText`) (`KismetStringLibrary.BuildString_Int` "" "Score: " (`self.Score`))) ; Update text
)

(fn `Get Grid Block`
  (params (Movement :type String)))

(fn `Set Main Spaceship`
  (params (Spaceship :type "Actor Object Reference"))
  (set `self.Main Spaceship` Spaceship))

(fn `UserConstructionScript`)