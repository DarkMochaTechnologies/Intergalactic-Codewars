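; Player character Blueprint for a sailor, handling its camera view, player name and chat relay.
; On BeginPlay it becomes player 0's view target, stores the name from its PlayerState, then after a short delay casts the HUD to BP_Navigator_HUD without further action.
; Chat messages pass from UpdateChat through server and client events into the Chat object.
; GetPlayerName is a stub returning an empty string.
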(event `self.ReceiveBeginPlay`
  (`PlayerController.SetViewTargetWithBlend` (`GameplayStatics.GetPlayerController` 0) self 0.0 "VTBlend_Linear" 0.0 false)
  (bind _name (message `/Game/ChatSystem/Chat.Get Player Name` (`self.PlayerState`)))
  (set `self.Player Name` _name)
  (`KismetSystemLibrary.Delay` 0.5)
  (cast `/Game/Blueprints/BP_Navigator_HUD` (`PlayerController.GetHUD` (`GameplayStatics.GetPlayerController` 0))))

(event `Update(Client)`
  (params (message :type "/Game/ChatSystem/ChatMessageStruct Structure"))
  (`/Game/ChatSystem/ChatWindow.UpdateChat` (`self.Chat`) message))

(event `self.ReceiveActorBeginOverlap`
  (params (OtherActor :type "Actor Object Reference")))

(event `Update(Server)`
  (params (message :type "/Game/ChatSystem/ChatMessageStruct Structure"))
  (`self.Update(Client)` message))

(event `self.ReceiveTick`
  (params (DeltaSeconds :type "Float (single-precision)")))

(event `self.Update Chat`
  (params (Message :type "/Game/ChatSystem/ChatMessageStruct Structure"))
  (`self.Update(Server)` Message))

(fn `Get Player Name`
  (returns (Name :type String))
  (return ""))

(fn `UserConstructionScript`)